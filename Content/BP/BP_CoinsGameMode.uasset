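; Game mode for a coin game that tracks the score and manages the HUD, intro message, win screen and game-over screen.
; BeginPlay creates these widgets, shows the intro over the HUD once for five seconds, then clears all widgets and loops back to rebuild them.
; AddPoints updates the score text and fires the OnPointsAdded dispatcher.
; Win and game-over events swap in their menu, enable UI-only input with a cursor, and pause the game.
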(event `self.ReceiveBeginPlay`
  (bind _returnvalue (`|CreateWidget` "/Game/BP/BP_HUD.BP_HUD_C" :!label _label))
  (bind _output_get (set `self.UIRef` _returnvalue))
  (`UserWidget.AddToViewport` _output_get 0)
  (bind _returnvalue_2 (`|CreateWidget` "/Game/BP/GameOver.GameOver_C"))
  (set `self.GameOver` _returnvalue_2)
  (bind _returnvalue_3 (`|CreateWidget` "/Game/BP/WinMenu.WinMenu_C"))
  (set `self.Win Menu` _returnvalue_3)
  (`/Engine/EditorBlueprintResources/StandardMacros.DoOnce` false
    (:`Completed`
      (bind _returnvalue_4 (`|CreateWidget` "/Game/BP/BP_UserCommunicate.BP_UserCommunicate_C"))
      (`UserWidget.AddToViewport` _returnvalue_4 0)
      (`KismetSystemLibrary.Delay` 5.0)
      (`WidgetLayoutLibrary.RemoveAllWidgets`)
      (goto _label))))

(event `AddPoints`
  (params (Points :type Integer))
  (bind _output_get (set `self.Score` (+ (`self.Score`) Points)))
  (`/Game/BP/BP_HUD.UpdateScoreText` (`self.UIRef`) (`KismetTextLibrary.Conv_IntToText` _output_get))
  (`self.OnPointsAdded` (`self.Score`)))

(event `EventWinGame`
  (bind _returnvalue (`GameplayStatics.GetPlayerController` 0))
  ;[1 1 1] GameOver
  (`WidgetLayoutLibrary.RemoveAllWidgets`)
  (`UserWidget.AddToViewport` (`self.Win Menu`) 0)
  (`WidgetBlueprintLibrary.SetInputMode_UIOnlyEx` _returnvalue null)
  (set `PlayerController.bShowMouseCursor` true _returnvalue)
  (`GameplayStatics.SetGamePaused` true))

(event `EventGameOver`
  (bind _returnvalue (`GameplayStatics.GetPlayerController` 0))
  (`WidgetLayoutLibrary.RemoveAllWidgets`)
  (`UserWidget.AddToViewport` (`self.GameOver`) 0)
  (`WidgetBlueprintLibrary.SetInputMode_UIOnlyEx` _returnvalue null)
  (set `PlayerController.bShowMouseCursor` true _returnvalue)
  (`GameplayStatics.SetGamePaused` true))

(fn `UserConstructionScript`)